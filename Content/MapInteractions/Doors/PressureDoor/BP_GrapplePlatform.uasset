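; BP_GrapplePlatform is a pressure-switch-driven mover that slides its Door component once enough switches are active.
; SwitchActivated and SwitchDeactivated adjust the active switch count and compare it with the required number.
; Meeting the threshold plays the DoorActivation timeline, which sets the Door's relative Y location, while falling short reverses it from its current position.
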(event Custom|SwitchActivated
  (Math|Integer|IncrementInt (Variables|Default|GetPressureSwitchesActive)
    (:%20%20
      (if (>= (Variables|Default|GetPressureSwitchesActive) (Variables|Default|GetPressureSwitchesNeeded))
        (bind _doorposition (Timeline|DoorActivation Play)
          (:Update
            (Transformation|SetRelativeLocation (Variables|Default|GetDoor) (Math|Vector|MakeVector 0.0 _doorposition 0.0) false false)))
        (else
          (Timeline|DoorActivation Reverse))))))

(event Custom|SwitchDeactivated
  (Math|Integer|DecrementInt (Variables|Default|GetPressureSwitchesActive)
    (:%20%20
      (if (>= (Variables|Default|GetPressureSwitchesActive) (Variables|Default|GetPressureSwitchesNeeded))
        (bind _doorposition (Timeline|DoorActivation Play)
          (:Update
            (Transformation|SetRelativeLocation (Variables|Default|GetDoor) (Math|Vector|MakeVector 0.0 _doorposition 0.0) false false)))
        (else
          (Timeline|DoorActivation Reverse))))))

(event EventBeginPlay)

(event EventTick
  (params (DeltaSeconds :type Float%20%28single-precision%29)))

(fn ConstructionScript)