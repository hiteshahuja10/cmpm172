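; BP_AI is a simple enemy AI pawn with a health bar widget.
; Pawn sensing sets a "hasSeenPlayer?" blackboard key when it sees the third-person player character, leaving behavior to the AI controller's blackboard.
; A sphere overlap with the player subtracts a fixed amount of the AI's own Health.
; UpdateHealthBar copies Health into the UI_EnemyHealth widget at start and after each hit.
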(event OnSeePawn(PawnSensing)
  (params (Pawn :type Pawn%20Object%20Reference))
  (Utilities|Casting|CastToBP_ThirdPersonCharacter Pawn)
  (AI|Components|Blackboard|SetValueasBool (AI|GetBlackboard (AI|GetAIController self)) (Utilities|Name|MakeLiteralName "hasSeenPlayer?") true))

(event OnComponentBeginOverlap(Sphere)
  (params (OverlappedComponent :type Primitive%20Component%20Object%20Reference) (OtherActor :type Actor%20Object%20Reference) (OtherComp :type Primitive%20Component%20Object%20Reference) (OtherBodyIndex :type Integer) (bFromSweep :type Boolean) (SweepResult :type Hit%20Result%20Structure%20%28by%20ref%29))
  (bind _asbp_third_person_character (Utilities|Casting|CastToBP_ThirdPersonCharacter OtherActor))
  (Utilities|IsValid _asbp_third_person_character
    (:Is%20Valid
      (Variables|Default|SetHealth (- (Variables|Default|GetHealth) 1e+01))
      (CallFunction|UpdateHealthBar))))

(event EventBeginPlay
  (CallFunction|UpdateHealthBar))

(fn ConstructionScript)

(fn UpdateHealthBar
  (bind _asui_enemy_health (Utilities|Casting|CastToUI_EnemyHealth (UserInterface|GetUserWidgetObject (Variables|Default|GetHealthBar))))
  (Utilities|IsValid _asui_enemy_health
    (:Is%20Valid
      (Variables|/Game/UI/UI_EnemyHealth.UI_EnemyHealth_C|SetHealth _asui_enemy_health (Variables|Default|GetHealth))
      (return))))