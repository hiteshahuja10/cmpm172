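; BP_Door is a pressure-switch door that moves once enough switches are active.
; Switch events adjust an active count, and either one plays the DoorActivation timeline while the threshold is met, driving the door's relative Z.
; No path reverses the timeline.
; SpawnEnemy spawns a BP_AI at a hardcoded location only while DoorOpenCount, incremented on every timeline update, is still zero.
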(event Custom|SpawnEnemy
  (if (== (Variables|Default|GetDoorOpenCount) 0)
    (AI|SpawnAIFromClass "/Game/Simple_AI/BP_AI.BP_AI_C" "/Game/Simple_AI/BT_AI.BT_AI" "-11730.000000,-91890.000000,7180.000000" "0, 0, 0" true 0)))

(event Custom|SwitchDeactivated
  (Math|Integer|DecrementInt (Variables|Default|GetPressureSwitchesActive)
    (:%20%20
      (if (>= (Variables|Default|GetPressureSwitchesActive) (Variables|Default|GetPressureSwitchesNeeded))
        (bind _doorposition (Timeline|DoorActivation Play)
          (:Update
            (Transformation|SetRelativeLocation (Variables|Default|GetDoor) (Math|Vector|MakeVector 0.0 0.0 _doorposition) false false)
            (Math|Integer|IncrementInt (Variables|Default|GetDoorOpenCount))))))))

(event Custom|SwitchActivated
  (Math|Integer|IncrementInt (Variables|Default|GetPressureSwitchesActive)
    (:%20%20
      (if (>= (Variables|Default|GetPressureSwitchesActive) (Variables|Default|GetPressureSwitchesNeeded))
        (bind _doorposition (Timeline|DoorActivation Play)
          (:Update
            (Transformation|SetRelativeLocation (Variables|Default|GetDoor) (Math|Vector|MakeVector 0.0 0.0 _doorposition) false false)
            (Math|Integer|IncrementInt (Variables|Default|GetDoorOpenCount))))))))

(event EventBeginPlay)

(event EventTick
  (params (DeltaSeconds :type Float%20%28single-precision%29)))

(fn ConstructionScript)