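; BP_RespawnCubes is a map interaction that resets four cubes to stored positions.
; On BeginPlay it moves each cube to its matching Pos variable in world space.
; Its Collision component repeats the same placement when overlapped by BP_Hero_Quinn_Child_P1, ignoring actors that fail that cast.
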(event OnComponentBeginOverlap(Collision)
  (params (OverlappedComponent :type Primitive%20Component%20Object%20Reference) (OtherActor :type Actor%20Object%20Reference) (OtherComp :type Primitive%20Component%20Object%20Reference) (OtherBodyIndex :type Integer) (bFromSweep :type Boolean) (SweepResult :type Hit%20Result%20Structure%20%28by%20ref%29))
  (Utilities|Casting|CastToBP_Hero_Quinn_Child_P1 OtherActor)
  (Transformation|SetWorldLocation (Variables|Default|GetCube1) (Variables|Default|GetPos1) false false)
  (Transformation|SetWorldLocation (Variables|Default|GetCube2) (Variables|Default|GetPos2) false false)
  (Transformation|SetWorldLocation (Variables|Default|GetCube3) (Variables|Default|GetPos3) false false)
  (Transformation|SetWorldLocation (Variables|Default|GetCube4) (Variables|Default|GetPos4) false false))

(event EventBeginPlay
  (Transformation|SetWorldLocation (Variables|Default|GetCube1) (Variables|Default|GetPos1) false false)
  (Transformation|SetWorldLocation (Variables|Default|GetCube2) (Variables|Default|GetPos2) false false)
  (Transformation|SetWorldLocation (Variables|Default|GetCube3) (Variables|Default|GetPos3) false false)
  (Transformation|SetWorldLocation (Variables|Default|GetCube4) (Variables|Default|GetPos4) false false))

(event EventTick
  (params (DeltaSeconds :type Float%20%28single-precision%29)))

(fn ConstructionScript)