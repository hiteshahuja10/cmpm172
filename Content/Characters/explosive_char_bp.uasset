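; Character Blueprint for a shooter character that fires explosive bubble projectiles and tracks aim-down-sights state.
; ADS input sets IsADS while held, and a custom event also sets it from a parameter.
; FireWeapon plays muzzle flash and pistol sound, then spawns an Explosivebubble at the weapon mesh's Muzzle socket.
; Impulse and line trace nodes are present but unconnected, so the character applies no launch force itself.
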(event Custom|CustomEvent
  (params (IsADS :type Boolean))
  (Variables|Default|SetIsADS IsADS))

(event Input|ActionEvents|InputActionADS
  (params (Key :type Key%20Structure))
  (:Pressed
    (Variables|Default|SetIsADS true))
  (:Released
    (Variables|Default|SetIsADS false)))

(event Input|ActionEvents|InputActionFireWeapon
  (params (Key :type Key%20Structure))
  (bind _weaponmesh (Variables|Default|GetWeaponMesh))
  (bind _returnvalue (Transformation|GetSocketTransform _weaponmesh "Muzzle" "RTS_World"))
  (:Pressed
    (Effects|SpawnEmitterAttached "/Game/MilitaryWeapSilver/FX/P_Pistol_MuzzleFlash_01.P_Pistol_MuzzleFlash_01" (Variables|Default|GetWeaponMesh) "Muzzle" "0, 0, 0" "0, 0, 0" "1.000000,1.000000,1.000000" "SnapToTarget")
    (Audio|PlaySound2D "/Game/MilitaryWeapSilver/Sound/Pistol/Cues/PistolA_Fire_Cue.PistolA_Fire_Cue" 1.0 1.0 0.0 0 0)
    (bind _returnvalue_2 (Game|SpawnActorfromClass "/Game/Characters/explosivebubble.explosivebubble_C" (Math|Transform|MakeTransform (.location _returnvalue) (.rotation _returnvalue) "1.000000,1.000000,1.000000") "Undefined" 0 0))))

(fn ConstructionScript
  (|CallParentFunction))