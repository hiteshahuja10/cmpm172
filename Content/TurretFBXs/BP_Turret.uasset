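; Auto-aiming turret that targets the nearest visible BP_Hero_Quinn pawn within sensing range and shoots it.
; Each tick, a sphere overlap with line-of-sight checks picks the target, then the top rotates toward it with clamped pitch.
; Once the cooldown has elapsed and a dot product confirms alignment, it spawns bullets from the left then right barrel sockets.
; Curve-driven timelines supply each barrel's recoil.
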(event Custom|Fire
  (Variables|Private|SetTimeOfLastFire (Utilities|Time|GetGameTimeinSeconds))
  (Utilities|FlowControl|Sequence ; Reset and Start   restart?
    (:then_0
      (goto _label Reset))
    (:then_1
      (Utilities|FlowControl|DoN 1 :!label _label ; Does something certain amount of time
        (:Exit
          (Game|SpawnActorfromClass "/Game/TurretFBXs/TurretBullet.TurretBullet_C" (Transformation|GetSocketTransform (Variables|Default|GetLeftBarrel) "FireSocket" "RTS_World") "Undefined" 0 0)
          (Components|Timeline|PlayfromStart (Variables|Default|GetRecoilTimeLineL))
          (Utilities|FlowControl|Delay 0.2)
          (Game|SpawnActorfromClass "/Game/TurretFBXs/TurretBullet.TurretBullet_C" (Transformation|GetSocketTransform (Variables|Default|GetRightBarrel) "FireSocket" "RTS_World") "Undefined" 0 0)
          (Components|Timeline|PlayfromStart (Variables|Default|GetRecoilTimeLineR))
          (Utilities|FlowControl|Delay 0.2)
          (goto _label))))))

(event EventTick
  (params (DeltaSeconds :type Float%20%28single-precision%29))
  (Private|FindBestTarget)
  (Variables|Private|GetTarget
    (:then
      (Private|UpdateTurretLocation DeltaSeconds)
      (Private|UpdateFire))
    (:else)))

(event EventBeginPlay
  (Class|TimelineComponent|SetFloatCurve (Variables|Default|GetRecoilTimeLineL) "/Game/TurretFBXs/RecoilCurve.RecoilCurve" "Recoil")
  (Class|TimelineComponent|SetFloatCurve (Variables|Default|GetRecoilTimeLineR) "/Game/TurretFBXs/RecoilCurve.RecoilCurve" "Recoil"))

(fn ConstructionScript)

(fn FindBestTarget
  (LocalVariables|SetBestDistance (+ (Variables|Constrants|GetSensingRange) 1.0))
  (bind _outactors (Collision|SphereOverlapActors (Transformation|GetActorLocation) (Variables|Constrants|GetSensingRange) (Utilities|Array|MakeArray "ObjectTypeQuery3") "/Game/Characters/BP_Hero_Quinn.BP_Hero_Quinn_C"))
  (for _array_element _outactors
    (bind _output_get (LocalVariables|SetCurrentTarget _array_element))
    (bind _output_get_2 (LocalVariables|SetCurrentDistance (Transformation|GetDistanceTo _output_get self)))
    (if (or (< _output_get_2 (LocalVariables|GetBestDistance)) (not (Utilities|IsValid (LocalVariables|GetBestTarget))))
      ;[1 1 1] If it had line of sight
      (bind _result (CallFunction|HasLineOfSight (Transformation|GetWorldLocation (Variables|Default|GetTop)) (Transformation|GetActorLocation (LocalVariables|GetCurrentTarget)) (Utilities|Array|MakeArray self (LocalVariables|GetCurrentTarget))))
      (if _result
        (LocalVariables|SetBestTarget (LocalVariables|GetCurrentTarget))
        (LocalVariables|SetBestDistance (LocalVariables|GetCurrentDistance)))))
  (Variables|Private|SetTarget (LocalVariables|GetBestTarget)))

(fn UpdateTurretLocation
  (params (DeltaSeconds :type Float%20%28double-precision%29))
  (bind _output_get (LocalVariables|SetNewLocalVar (Class|KismetMathLibrary|RInterptoConstant (Transformation|GetWorldRotation (Variables|Default|GetTop)) (Math|Rotator|FindLookatRotation (Transformation|GetWorldLocation (Variables|Default|GetTop)) (Transformation|GetActorLocation (Variables|Private|GetTarget))) DeltaSeconds (Variables|Constrants|GetInterp%20Speed))))
  (Transformation|SetWorldRotation (Variables|Default|GetTop) (Math|Rotator|MakeRotator (.roll _output_get) (Math|Float|ClampAngle (.pitch _output_get) -45.0 75.0) (.yaw _output_get)) false false))

(fn UpdateFire
  (if (> (- (Utilities|Time|GetGameTimeinSeconds) (Variables|Private|GetTimeOfLastFire)) (Variables|Constrants|GetRateOfFire)) ; cool down
    (if (> (Math|Vector|DotProduct (Math|Vector|GetUnitDirection(Vector) (Transformation|GetWorldLocation (Variables|Default|GetTop)) (Transformation|GetActorLocation (Variables|Private|GetTarget))) (Math|Vector|GetForwardVector (Variables|Default|GetTop))) 0.999) ; Facing Target?
      (CallFunction|Fire))))